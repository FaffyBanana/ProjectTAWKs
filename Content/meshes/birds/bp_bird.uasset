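; Bird actor that animates a flapping mesh and moves it along its local X axis.
; On BeginPlay, a timeline drives the "Key 1" morph target on BirdSolo from its WingSpeed track, scaled by a small random factor on every update.
; A second timeline, played from Tick, sets the mesh's relative X location from its negated Location track, with sweep and teleport enabled.
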(event EventBeginPlay
  (Variables|Default|SetOriginal%20Location (Variables|Default|GetOriginal%20Location))
  (Utilities|FlowControl|Sequence
    (:then_0
      (bind _wingspeed (Timeline|Timeline_0 Play)
        (:Update
          (Components|SkeletalMesh|SetMorphTarget (Variables|Default|Getbird__solo) "Key 1" (* _wingspeed (Math|Random|RandomFloatinRange 0.8 1.0)) true))))))

(event EventTick
  (params (DeltaSeconds :type Float%20%28single-precision%29))
  (bind _location (Timeline|Timeline_1 Play)
    (:Update
      (Transformation|SetRelativeLocation (Variables|Default|Getbird__solo) (Math|Vector|MakeVector (* _location -1.0) 0.0 0.0) true true))))

(fn ConstructionScript)